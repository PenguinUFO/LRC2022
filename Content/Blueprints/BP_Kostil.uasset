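; BP_Kostil is a trigger box actor that acts on overlaps with the companion or an enemy character.
; When a BP_Companion enters the box, it prints a long-lasting debug message and moves the companion to just above player 0's character.
; When a BP_CharEmeny enters, the box actor moves itself to just above that enemy, rather than moving the enemy.
; Both checks match the exact class, and both moves skip sweeping.
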(event OnComponentBeginOverlap(Box)
  (params (OverlappedComponent :type Primitive%20Component%20Object%20Reference) (OtherActor :type Actor%20Object%20Reference) (OtherComp :type Primitive%20Component%20Object%20Reference) (OtherBodyIndex :type Integer) (bFromSweep :type Boolean) (SweepResult :type Hit%20Result%20Structure%20%28by%20ref%29))
  (bind _returnvalue (Utilities|GetClass OtherActor))
  (if (== _returnvalue "/Game/Blueprints/BP_Companion.BP_Companion_C")
    (Development|PrintString "stop right there criminal ball!!" true true "(R=0.909453,G=0.000000,B=1.000000,A=1.000000)" 2e+01)
    (Transformation|SetActorLocation OtherActor (+ (Transformation|GetActorLocation (Game|GetPlayerCharacter 0)) "0,0,150.000000") false false)
    (elif (== _returnvalue "/Game/Evgeniy/Enemies/Enemy/BP_CharEmeny.BP_CharEmeny_C")
      (Transformation|SetActorLocation (+ (Transformation|GetActorLocation OtherActor) "0,0,100.000000") false false))))

(event EventBeginPlay)

(event Collision|EventActorBeginOverlap
  (params (OtherActor :type Actor%20Object%20Reference)))

(event EventTick
  (params (DeltaSeconds :type Float%20%28single-precision%29)))

(fn ConstructionScript)