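; Point light actor that can be dimmed or triggered to flicker in a short burst.
; BeginPlay stores the starting intensity, and SwitchLight toggles between that value and a fixed dimmed level.
; EnableFlicker sets a flag that Tick picks up to run FlickerLights, which clears the flag and calls SwitchLight four times with short random delays, leaving the light in its prior dim state.
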(event EventBeginPlay
  (Variables|Default|SetintensityStored (Variables|/Script/Engine.LightComponentBase|GetIntensity (Variables|Default|GetPointLight))))

(event Collision|EventActorBeginOverlap
  (params (OtherActor :type Actor%20Object%20Reference)))

(event EventTick
  (params (DeltaSeconds :type Float%20%28single-precision%29))
  (if (Variables|Default|GetisFlickering)
    (Utilities|FlickerLights)))

(fn ConstructionScript)

(fn SwitchLight
  (bind _pointlight (Variables|Default|GetPointLight))
  (if (Variables|Default|GetisDimmed)
    (Rendering|Components|Light|SetIntensity _pointlight (Variables|Default|GetintensityStored))
    (Variables|Default|SetisDimmed false)
    (else
      (Rendering|Components|Light|SetIntensity _pointlight 5e+02)
      (Variables|Default|SetisDimmed true))))

(fn EnableFlicker
  (Variables|Default|SetisFlickering true))