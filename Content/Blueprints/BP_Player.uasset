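; Player Blueprint that can tether a BP_Companion with a cable rope and grab it through a physics handle.
; GrabComponent has the companion's own PhysicsHandle grab its mesh, then attaches the Cable end to it.
; DropCompanion calls the same grab with no component instead of an explicit release, then detaches the cable.
; The event graph is inactive: its drop call and debug print are unreachable.
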(event EventBeginPlay)

(event Collision|EventActorBeginOverlap
  (params (OtherActor :type Actor%20Object%20Reference)))

(event EventTick
  (params (DeltaSeconds :type Float%20%28single-precision%29)))

(fn ConstructionScript)

(fn GrabComponent
  (params (Companion :type BP%20Companion%20Object%20Reference))
  (Class|PhysicsHandleComponent|GrabComponentatLocation (Variables|/Game/Blueprints/BP_Companion.BP_Companion_C|GetPhysicsHandle Companion) (Variables|/Game/Blueprints/BP_Companion.BP_Companion_C|GetMesh Companion) "None" (Transformation|GetWorldLocation (Variables|/Script/Engine.Actor|GetRootComponent Companion)))
  (CallFunction|AttachRope Companion))

(fn DropCompanion
  (params (Companion :type BP%20Companion%20Object%20Reference))
  (Class|PhysicsHandleComponent|GrabComponentatLocation (Variables|/Game/Blueprints/BP_Companion.BP_Companion_C|GetPhysicsHandle Companion) 0 "None" "0, 0, 0")
  (CallFunction|DetachRope))

(fn AttachRope
  (params (Companion :type BP%20Companion%20Object%20Reference))
  (bind _cable (Variables|Default|GetCable))
  (Class|CableComponent|SetAttachEndto _cable Companion "None" "None")
  (Variables|/Script/CableComponent.CableComponent|SetbAttachEnd _cable true))

(fn DetachRope
  (bind _cable (Variables|Default|GetCable))
  (Class|CableComponent|SetAttachEndto _cable 0 "None" "None")
  (Variables|/Script/CableComponent.CableComponent|SetbAttachEnd _cable false))