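; Helper actor for a magnet power-up that pulls one Orb toward the Hero.
; Each Tick, the DistanceIsOk macro checks that their distance lies between a small fixed minimum and MaxDistance.
; In range, it adds a velocity-change impulse to the Orb's mesh along ToHeroVector, scaled by MagnetPower but not delta time.
; Out of range, it clears the Orb's ImMagneted flag and destroys itself.
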(event EventBeginPlay)

(event Collision|EventActorBeginOverlap
  (params (OtherActor :type Actor%20Object%20Reference)))

(event EventTick
  (params (DeltaSeconds :type Float%20%28single-precision%29))
  (Utilities|DistanceIsOk
    (:In%20Range
      (Physics|AddImpulse (Variables|/Game/Blueprints/BP_Companion.BP_Companion_C|GetMesh (Variables|Default|GetOrb)) (* (CallFunction|ToHeroVector) (Variables|Default|GetMagnetPower)) "None" true))))

(fn ConstructionScript)

(fn ToHeroVector
  (return (Math|Vector|GetUnitDirection(Vector) (Transformation|GetActorLocation (Variables|Default|GetOrb)) (Transformation|GetActorLocation (Variables|Default|GetHero)))))