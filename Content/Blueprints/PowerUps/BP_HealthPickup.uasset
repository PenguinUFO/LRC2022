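; BP_HealthPickup is a health power-up that heals the player when they touch it.
; A sphere overlap casts the other actor to BP_Player and checks its health system component, doing nothing if HP is already full.
; Otherwise it applies the Heal amount, refreshes the player's HUD HP, plays a heal sound at its location and destroys itself.
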(event OnComponentBeginOverlap(Sphere)
  (params (OverlappedComponent :type Primitive%20Component%20Object%20Reference) (OtherActor :type Actor%20Object%20Reference) (OtherComp :type Primitive%20Component%20Object%20Reference) (OtherBodyIndex :type Integer) (bFromSweep :type Boolean) (SweepResult :type Hit%20Result%20Structure%20%28by%20ref%29))
  (bind _asbp_player (Utilities|Casting|CastToBP_Player OtherActor))
  (if (not (Default|IsFullHP (Variables|/Game/Blueprints/BP_Player.BP_Player_C|GetBP_CC_HealthSystem _asbp_player)))
    (Default|TakeHeal (Variables|/Game/Blueprints/BP_Player.BP_Player_C|GetBP_CC_HealthSystem _asbp_player) (Variables|Default|GetHeal))
    (Default|UpdateHUDHP _asbp_player (Variables|/Game/Evgeniy/Enemies/BP_CC_HealthSystem.BP_CC_HealthSystem_C|GetCurrentHP (Variables|/Game/Blueprints/BP_Player.BP_Player_C|GetBP_CC_HealthSystem _asbp_player)))
    (Audio|PlaySoundatLocation "/Game/SoundFX/PickUps/heal/Healup.Healup" (Transformation|GetActorLocation) "0, 0, 0" 1.0 1.0 0.0 0 0 0 0)
    (Actor|DestroyActor)))

(event EventBeginPlay)

(event Collision|EventActorBeginOverlap
  (params (OtherActor :type Actor%20Object%20Reference)))

(event EventTick
  (params (DeltaSeconds :type Float%20%28single-precision%29)))

(fn ConstructionScript)