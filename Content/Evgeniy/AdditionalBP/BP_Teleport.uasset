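; BP_Teleport is a trigger volume that moves the player to a destination, presented as an elevator ride.
; On player overlap it plays an ascending sound and adds a centered IntoTheDark widget to the main HUD, then relocates the player after a short delay.
; After a longer delay it plays a bell and moves the controller's TrueCompanion to its own destination.
; The construction script scales the box from per-instance Y and Z variables with a fixed X.
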(event OnComponentBeginOverlap(Box)
  (params (OverlappedComponent :type Primitive%20Component%20Object%20Reference) (OtherActor :type Actor%20Object%20Reference) (OtherComp :type Primitive%20Component%20Object%20Reference) (OtherBodyIndex :type Integer) (bFromSweep :type Boolean) (SweepResult :type Hit%20Result%20Structure%20%28by%20ref%29))
  (bind _asbp_player (Utilities|Casting|CastToBP_Player OtherActor))
  (Audio|PlaySoundatLocation "/Game/SoundFX/Teleport/ElevatorAscending.ElevatorAscending" (Transformation|GetActorLocation _asbp_player) "0, 0, 0" 1.0 1.0 0.0 0 0 0 0) ; Elevator sound
  (bind _returnvalue (UserInterface|CreateWidget "/Game/HUD/HUD_IntoTheDark.HUD_IntoTheDark_C" (Game|GetPlayerController 0)))
  (bind _returnvalue_2 (Class|CanvasPanel|AddChildtoCanvas (Variables|/Game/HUD/HUD_Main.HUD_Main_C|GetCanvasPanel (Variables|/Game/Blueprints/BP_Player.BP_Player_C|GetMainHUD _asbp_player)) _returnvalue))
  (Class|CanvasPanelSlot|SetAutoSize _returnvalue_2 true)
  (Class|CanvasPanelSlot|SetAlignment _returnvalue_2 "(X=0.500000,Y=0.500000)")
  (Class|CanvasPanelSlot|SetAnchors _returnvalue_2 (Utilities|Struct|MakeAnchors "(X=0.500000,Y=0.500000)" "(X=0.500000,Y=0.500000)"))
  (Utilities|FlowControl|Delay 1.1)
  (Transformation|SetActorLocation _asbp_player (Variables|Default|GetDestination) false false)
  (Utilities|FlowControl|Delay 23.0)
  (Audio|PlaySoundatLocation "/Game/SoundFX/Teleport/Elevator_bell_small_001.Elevator_bell_small_001" (Transformation|GetActorLocation _asbp_player) "0, 0, 0" 1.0 1.0 0.0 0 0 0 0) ; Elevator sound
  (bind _asbp_side_scroller_controller (Utilities|Casting|CastToBP_SIdeScrollerController (Game|GetPlayerController 0)))
  (Transformation|SetActorLocation (Variables|/Game/Blueprints/BP_SIdeScrollerController.BP_SIdeScrollerController_C|GetTrueCompanion _asbp_side_scroller_controller) (Variables|Default|GetCompanionDestination) false false))

(event EventBeginPlay)

(event Collision|EventActorBeginOverlap
  (params (OtherActor :type Actor%20Object%20Reference)))

(event EventTick
  (params (DeltaSeconds :type Float%20%28single-precision%29)))

(fn ConstructionScript
  (Transformation|SetWorldScale3D (Variables|Default|GetBox) (Math|Vector|MakeVector 3.0 (Variables|Default|GetBoxY) (Variables|Default|GetBoxZ))))