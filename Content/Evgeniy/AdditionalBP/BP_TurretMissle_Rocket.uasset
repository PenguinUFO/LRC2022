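; Turret missile rocket Blueprint that tracks which actors are inside its explosion area.
; The construction script scales ExplosionCollision by ExplosionRadius, and that component's begin and end overlap events add and remove actors in ActorsInExplosionArea without duplicates.
; When the rocket overlaps an actor, it calls the parent handler, then prints a "Damaging" message for each listed actor without applying damage itself.
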(event OnComponentBeginOverlap(ExplosionCollision)
  (params (OverlappedComponent :type Primitive%20Component%20Object%20Reference) (OtherActor :type Actor%20Object%20Reference) (OtherComp :type Primitive%20Component%20Object%20Reference) (OtherBodyIndex :type Integer) (bFromSweep :type Boolean) (SweepResult :type Hit%20Result%20Structure%20%28by%20ref%29))
  (CallFunction|AddActortoActorsinExplosionZoneList OtherActor))

(event OnComponentEndOverlap(ExplosionCollision)
  (params (OverlappedComponent :type Primitive%20Component%20Object%20Reference) (OtherActor :type Actor%20Object%20Reference) (OtherComp :type Primitive%20Component%20Object%20Reference) (OtherBodyIndex :type Integer))
  (CallFunction|RemoveActorfromActorsinExplosionZoneList OtherActor))

(event EventBeginPlay
  (|CallParentFunction) ; This node is disabled and will not be called.\nDrag off pins to build functionality.
)

(event Collision|EventActorBeginOverlap
  (params (OtherActor :type Actor%20Object%20Reference))
  (|CallParentFunction OtherActor)
  (for _array_element (Variables|Default|GetActorsInExplosionArea)
    (Development|PrintString (Utilities|String|ToString(Text) (Utilities|Text|FormatText "Damaging the {actor}" _array_element)))))

(event EventTick
  (params (DeltaSeconds :type Float%20%28single-precision%29))
  (|CallParentFunction DeltaSeconds) ; This node is disabled and will not be called.\nDrag off pins to build functionality.
)

(fn ConstructionScript
  (|CallParentFunction)
  (Transformation|SetRelativeScale3D (Variables|Default|GetExplosionCollision) (Math|Conversions|ToVector(Float) (Variables|Default|GetExplosionRadius))))

(fn AddActortoActorsinExplosionZoneList
  (params (NearbyActor :type Actor%20Object%20Reference%20%28by%20ref%29))
  (if (not (Utilities|Array|ContainsItem (Variables|Default|GetActorsInExplosionArea) NearbyActor))
    (Utilities|Array|Add (Variables|Default|GetActorsInExplosionArea) NearbyActor)))

(fn RemoveActorfromActorsinExplosionZoneList
  (params (NearbyActor :type Actor%20Object%20Reference%20%28by%20ref%29))
  (if (Utilities|Array|ContainsItem (Variables|Default|GetActorsInExplosionArea) NearbyActor)
    (Utilities|Array|RemoveItem (Variables|Default|GetActorsInExplosionArea) NearbyActor)))