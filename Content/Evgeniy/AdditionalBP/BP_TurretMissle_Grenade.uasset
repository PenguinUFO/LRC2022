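; Grenade projectile for a turret, with a blinking light and area-damage logic.
; BeginPlay loops a Delay and FlipFlop to toggle the PointLight; the Delay's zero exponent ignores the computed cycle time, yielding one second.
; MakeExplosion sphere-traces at the grenade and passes hit actors, except components tagged NotForHit, to the parent's MakeAHit.
; The explode, spawn BP_Explosion and destroy chain is unconnected; helpers maintain an explosion-area actor list that the trace ignores.
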(event EventBeginPlay
  (bind _pointlight (Variables|Default|GetPointLight))
  (|CallParentFunction)
  (Variables|Default|SetFirstCycle (/ (Variables|Default|GetTimer) (Variables|Default|GetCycleCount)))
  (for _index (range 1 (Variables|Default|GetCycleCount))
    (Utilities|FlowControl|Delay (Math|Float|Power (Variables|Default|GetFirstCycle) 0.0))
    (Utilities|FlowControl|FlipFlop
      (:A
        (Rendering|Components|Light|SetIntensity _pointlight 0.0))
      (:B
        (Rendering|Components|Light|SetIntensity _pointlight (Variables|Default|GetLightIntens))))))

(fn ConstructionScript
  (|CallParentFunction))

(fn AddActortoActorsinExplosionZoneList
  (params (NearbyActor :type Actor%20Object%20Reference%20%28by%20ref%29))
  (if (not (Utilities|Array|ContainsItem (Variables|Default|GetActorsInExplosionArea) NearbyActor))
    (Utilities|Array|Add (Variables|Default|GetActorsInExplosionArea) NearbyActor)))

(fn RemoveActorfromActorsinExplosionZoneList
  (params (NearbyActor :type Actor%20Object%20Reference%20%28by%20ref%29))
  (if (Utilities|Array|ContainsItem (Variables|Default|GetActorsInExplosionArea) NearbyActor)
    (Utilities|Array|RemoveItem (Variables|Default|GetActorsInExplosionArea) NearbyActor)))

(fn MakeExplosion
  (bind _returnvalue (Transformation|GetActorLocation))
  (bind _outhits (Collision|MultiSphereTraceByChannel _returnvalue _returnvalue (Variables|Default|GetExplosionRadius) "TraceTypeQuery1" false 0 "None"))
  (for _array_element _outhits
    (if (not (Components|ComponentHasTag (.HitComponent (Collision|BreakHitResult _array_element)) "NotForHit"))
      (CallFunction|MakeAHit (.HitActor (Collision|BreakHitResult _array_element))))))

(fn MakeAHit
  (params (DamagedActor :type Actor%20Object%20Reference))
  (|CallParentFunction DamagedActor))