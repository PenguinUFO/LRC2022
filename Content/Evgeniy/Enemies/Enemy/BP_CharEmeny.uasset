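; Enemy character that damages the player on touch and is set up to respawn after being destroyed.
; Incoming damage goes to BPCCHealthSystem, while capsule overlap applies physical damage to the player and pauses overlap events for a stun delay.
; Destruction starts a timer on itself to spawn the same class at its capsule location.
; Construction records spawn point and mesh scale, both unused in this graph.
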(event OnComponentBeginOverlap(Capsule)
  (params (OverlappedComponent :type Primitive%20Component%20Object%20Reference) (OtherActor :type Actor%20Object%20Reference) (OtherComp :type Primitive%20Component%20Object%20Reference) (OtherBodyIndex :type Integer) (bFromSweep :type Boolean) (SweepResult :type Hit%20Result%20Structure%20%28by%20ref%29))
  (if (== OtherActor (Game|GetPlayerCharacter 0))
    (Variables|/Script/Engine.PrimitiveComponent|SetbGenerateOverlapEvents (Variables|Default|GetCapsule) false)
    (Game|Damage|ApplyDamage OtherActor (Variables|Default|GetTouchDamage) 0 self "/Game/Evgeniy/Enemies/BP_PhysicDamage.BP_PhysicDamage_C")
    (Utilities|FlowControl|Delay (Variables|Default|GetStunDurationAfterAttack))
    (Variables|/Script/Engine.PrimitiveComponent|SetbGenerateOverlapEvents (Variables|Default|GetCapsule) true)))

(event Custom|Respawn
  (bind _self self)
  (Game|SpawnActorfromClass (Utilities|GetClass _self) (Math|Transform|MakeTransform (Transformation|GetWorldLocation (Variables|Collision|GetCapsuleComponent _self)) "0, 0, 0" "1.000000,1.000000,1.000000") "Undefined" 0 0))

(event EventBeginPlay)

(event Collision|EventActorBeginOverlap
  (params (OtherActor :type Actor%20Object%20Reference)))

(event EventTick
  (params (DeltaSeconds :type Float%20%28single-precision%29)))

(event EventDestroyed
  (Utilities|Time|SetTimerbyEvent (delegate Custom|Respawn) (Variables|Default|GetRespawn%20Timer)) ; Когда умирает, надо его возродить через заданное время
)

(event Game|Damage|EventAnyDamage
  (params (Damage :type Float%20%28single-precision%29) (DamageType :type Damage%20Type%20Object%20Reference) (InstigatedBy :type Controller%20Object%20Reference) (DamageCauser :type Actor%20Object%20Reference))
  (Default|TakeDamage (Variables|Default|GetBP_CC_HealthSystem) Damage))

(fn ConstructionScript
  (Variables|Default|SetSpawnPoint (Transformation|GetWorldLocation (Variables|Collision|GetCapsuleComponent)))
  (Variables|Default|SetInitialSize (Transformation|GetWorldScale (Variables|Character|GetMesh))))