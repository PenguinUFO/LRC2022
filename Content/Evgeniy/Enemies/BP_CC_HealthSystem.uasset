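; BP_CC_HealthSystem is a health component, stored with the enemy assets, that tracks damage and destroys its owner at zero health.
; TakeDamage subtracts damage from CurrentHP, clamps the result between zero and MaxHP, and calls KillCharacter when it reaches zero.
; KillCharacter destroys the owning actor immediately, and the event graph holds only disabled placeholder events.
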(event EventBeginPlay)

(event EventTick
  (params (DeltaSeconds :type Float%20%28single-precision%29)))

(fn TakeDamage
  (params (Damage :type Float%20%28double-precision%29))
  (bind _output_get (Variables|Default|SetCurrentHP (Math|Float|Clamp(Float) (- (Variables|Default|GetCurrentHP) Damage) 0.0 (Variables|Default|GetMaxHP))))
  (if (== _output_get 0.0)
    (CallFunction|KillCharacter)))

(fn KillCharacter
  (Actor|DestroyActor (Components|GetOwner)))