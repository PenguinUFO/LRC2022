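; Door actor that swings a static mesh open and closed around its yaw, triggered by inherited DoIt and UndoIt overrides that both call TurnIt.
; TurnIt ignores calls while moving, alternates direction with a FlipFlop, plays a sound and disables mesh collision.
; A timeline feeds NewDoorDegree, which offsets yaw from the starting rotation, then collision returns on finish.
; OpenOrClose offers an instant rotation but is not called here.
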(event Custom|TurnIt
  (bind _staticmesh (Variables|Default|GetStaticMesh))
  (if (not (Variables|Default|GetInMovement))
    (bind _isa (Utilities|FlowControl|FlipFlop)
      (:A
        _)
      (:B
        _))
    (Variables|Default|SetOpening _isa)
    (Variables|Default|SetInMovement true)
    (Collision|SetCollisionEnabled _staticmesh "NoCollision")
    (Variables|Default|SetInitialRotation (Variables|/Script/Engine.SceneComponent|GetRelativeRotation _staticmesh))
    (Audio|PlaySoundatLocation (Variables|Default|GetNoiseSounds) (Transformation|GetWorldLocation (Variables|Default|GetDefaultSceneRoot)) "0, 0, 0" 1.0 1.0 0.0 0 0 0 0)
    (bind _doordegree (Timeline|Timeline_0 PlayFromStart)
      (:Update
        (CallFunction|NewDoorDegree _doordegree))
      (:Finished
        (Variables|Default|SetInMovement false)
        (Collision|SetCollisionEnabled (Variables|Default|GetStaticMesh) "QueryAndPhysics")))))

(event EventBeginPlay
  (|CallParentFunction) ; This node is disabled and will not be called.\nDrag off pins to build functionality.
)

(event Collision|EventActorBeginOverlap
  (params (OtherActor :type Actor%20Object%20Reference))
  (|CallParentFunction OtherActor) ; This node is disabled and will not be called.\nDrag off pins to build functionality.
)

(event EventTick
  (params (DeltaSeconds :type Float%20%28single-precision%29))
  (|CallParentFunction DeltaSeconds) ; This node is disabled and will not be called.\nDrag off pins to build functionality.
)

(fn ConstructionScript
  (|CallParentFunction))

(fn OpenorClose
  (params (FlipOrFlop :type Boolean))
  (bind _initialrotation (Variables|Default|GetInitialRotation))
  (if FlipOrFlop
    (Transformation|SetRelativeRotation (Variables|Default|GetStaticMesh) (Math|Rotator|MakeRotator (.roll _initialrotation) (.pitch _initialrotation) (+ (.yaw _initialrotation) (Variables|Default|GetOpenDegree))) false false)
    (else
      (Transformation|SetRelativeRotation (Variables|Default|GetStaticMesh) (Variables|Default|GetInitialRotation) false false))))

(fn NewDoorDegree
  (params (DeltaDegree :type Float%20%28double-precision%29))
  (bind _initialrotation (Variables|Default|GetInitialRotation))
  (if (Variables|Default|GetOpening)
    (LocalVariables|SetDelta DeltaDegree)
    (else
      (LocalVariables|SetDelta (* DeltaDegree -1.0))))
  (Transformation|SetRelativeRotation (Variables|Default|GetStaticMesh) (Math|Rotator|MakeRotator (.roll _initialrotation) (.pitch _initialrotation) (+ (.yaw _initialrotation) (LocalVariables|GetDelta))) false false))

(fn DoIt
  (|CallParentFunction)
  (CallFunction|TurnIt))

(fn UndoIt
  (|CallParentFunction)
  (CallFunction|TurnIt))