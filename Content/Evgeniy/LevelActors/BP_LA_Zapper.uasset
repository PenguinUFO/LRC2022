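; BP_LA_Zapper is a level actor that knocks nearby BP_Companion actors away.
; Every tick it runs a debug-drawn multi-sphere trace around itself and picks out companions that are not magneted.
; For each, it makes the side-scroller player controller release any valid held companion, then applies a velocity-change impulse to the hit companion's mesh.
; PunchForce is negated when the companion's Y is below the zapper's.
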(event EventBeginPlay
  (|CallParentFunction) ; This node is disabled and will not be called.\nDrag off pins to build functionality.
)

(event Collision|EventActorBeginOverlap
  (params (OtherActor :type Actor%20Object%20Reference))
  (|CallParentFunction OtherActor) ; This node is disabled and will not be called.\nDrag off pins to build functionality.
)

(event EventTick
  (params (DeltaSeconds :type Float%20%28single-precision%29))
  (bind _returnvalue (Transformation|GetActorLocation))
  (bind _punchforce (Variables|Default|GetPunchForce))
  (|CallParentFunction DeltaSeconds)
  (bind _outhits (Collision|MultiSphereTraceByChannel _returnvalue _returnvalue 3e+02 "TraceTypeQuery1" false 0 "ForDuration" true "(R=1.000000,G=0.000000,B=0.000000,A=1.000000)" "(R=0.000000,G=1.000000,B=0.000000,A=1.000000)" 1.0))
  (for _array_element _outhits
    (bind _asbp_companion (Utilities|Casting|CastToBP_Companion (.HitActor (Collision|BreakHitResult _array_element))))
    (if (not (Variables|/Game/Blueprints/BP_Companion.BP_Companion_C|GetI'm%20Magneted _asbp_companion))
      (bind _asbp_side_scroller_controller (Utilities|Casting|CastToBP_SIdeScrollerController (Game|GetPlayerController 0)))
      (Variables|/Game/Blueprints/BP_SIdeScrollerController.BP_SIdeScrollerController_C|GetCompanion _asbp_side_scroller_controller
        (:then
          (Default|ReleaseCompanion _asbp_side_scroller_controller))
        (:else
          _))
      (if (< (.y (Transformation|GetActorLocation _asbp_companion)) (.y (Transformation|GetActorLocation)))
        (Physics|AddImpulse (Variables|/Game/Blueprints/BP_Companion.BP_Companion_C|GetMesh _asbp_companion) (* _punchforce -1.0) "None" true)
        (else
          (Physics|AddImpulse (Variables|/Game/Blueprints/BP_Companion.BP_Companion_C|GetMesh _asbp_companion) _punchforce "None" true))))))

(fn ConstructionScript
  (|CallParentFunction))