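; Destructible level object that shakes and plays a sound when damaged, and releases enemies when destroyed.
; BPCCHealthSystem handles damage, with HP, mesh and hidden-target tags set in the construction script.
; DestroyMe spawns one offset BP_CharEmeny with BT_Enemy per Loot entry, removes the actor, and optionally calls DoIt on linked SlaveActors.
; Its own DoIt destroys it without spawning, so another actor can remove it.
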(event Custom|Shake
  (bind _initial_location (Variables|Default|GetInitial%20Location))
  (bind _location (Timeline|ShakingTime PlayFromStart)
    (:Update
      (Transformation|SetWorldLocation (Variables|Default|GetStaticMesh) (Math|Vector|MakeVector (.x _initial_location) (+ (* _location (Variables|Default|GetShakeAmplitude)) (.y _initial_location)) (.z _initial_location)) false false))
    (:Finished
      (Transformation|SetActorLocation (Variables|Default|GetInitial%20Location) false false))))

(event EventBeginPlay
  (|CallParentFunction) ; This node is disabled and will not be called.\nDrag off pins to build functionality.
)

(event Collision|EventActorBeginOverlap
  (params (OtherActor :type Actor%20Object%20Reference))
  (|CallParentFunction OtherActor) ; This node is disabled and will not be called.\nDrag off pins to build functionality.
)

(event EventDestroyMe
  (bind _returnvalue (Transformation|GetActorLocation))
  (Audio|PlaySoundatLocation "/Game/SoundFX/LevelActors/DestructibleWall/WallDestroyed_Cue.WallDestroyed_Cue" (Variables|Default|GetInitial%20Location) "0, 0, 0" 1.0 1.0 0.0 0 0 0 0)
  (Utilities|FlowControl|Sequence
    (:then_0
      (for (_ _array_index) (Variables|Default|GetLoot)
        (AI|SpawnAIFromClass "/Game/Evgeniy/Enemies/Enemy/BP_CharEmeny.BP_CharEmeny_C" "/Game/Evgeniy/Enemies/Enemy/BT_Enemy.BT_Enemy" (Math|Vector|MakeVector (.x _returnvalue) (+ (* _array_index 50) (.y _returnvalue)) (.z _returnvalue)) "0, 0, 0" false 0))
      (Actor|DestroyActor))
    (:then_1
      (if (Variables|Default|GetDestroySlaves?)
        (for _array_element (Variables|Default|GetSlaveActor)
          (CallFunction|DoIt _array_element))))))

(event Game|Damage|EventAnyDamage
  (params (Damage :type Float%20%28single-precision%29) (DamageType :type Damage%20Type%20Object%20Reference) (InstigatedBy :type Controller%20Object%20Reference) (DamageCauser :type Actor%20Object%20Reference))
  (bind _playreactanimation (Default|TakeDamage (Variables|Default|GetBP_CC_HealthSystem) Damage DamageType DamageCauser))
  (if _playreactanimation
    (CallFunction|Shake)
    (Audio|PlaySoundatLocation "/Game/SoundFX/LevelActors/DestructibleWall/blockNoise_Cue.blockNoise_Cue" (Variables|Default|GetInitial%20Location) "0, 0, 0" 1.0 1.0 0.0 0 0 0 0)))

(fn ConstructionScript
  (bind _bp_cc_healthsystem (Variables|Default|GetBP_CC_HealthSystem))
  (bind _tags (Variables|Default|GetTags))
  (|CallParentFunction)
  (Utilities|FlowControl|Sequence
    (:then_0
      (Variables|Default|SetInitial%20Location (Transformation|GetActorLocation))
      (Variables|/Game/Evgeniy/Enemies/BP_CC_HealthSystem.BP_CC_HealthSystem_C|SetCurrentHP _bp_cc_healthsystem (Variables|Default|GetHP%20Current))
      (Variables|/Game/Evgeniy/Enemies/BP_CC_HealthSystem.BP_CC_HealthSystem_C|SetMaxHP _bp_cc_healthsystem (Variables|Default|GetHP%20Max)))
    (:then_1
      (bind _appearance (Variables|Default|GetAppearance)
        (:then
          (Components|StaticMesh|SetStaticMesh (Variables|Default|GetStaticMesh) _appearance))
        (:else)))
    (:then_2
      (if (Variables|Default|GetHiddenActor)
        (Utilities|Array|Add _tags "HiddenTarget")
        (Utilities|Array|RemoveItem _tags "BallTarget")))))

(fn Destroy
  (|CallParentFunction))

(fn DoIt
  (|CallParentFunction)
  (Actor|DestroyActor))