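; BP_LA_SpikedDemon is a spiked demon level actor that hurts what collides with its spikes and has an animated death.
; Hits on either of its two cone components pass the other actor to DealDamageFromSpikes, which is not defined in this graph.
; DestroyMe plays an alligator hiss, runs the Death timeline to scale the mesh relative to its current size, then destroys the actor.
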(event OnComponentHit(Cone1)
  (params (HitComponent :type Primitive%20Component%20Object%20Reference) (OtherActor :type Actor%20Object%20Reference) (OtherComp :type Primitive%20Component%20Object%20Reference) (NormalImpulse :type Vector :default "0, 0, 0") (Hit :type Hit%20Result%20Structure%20%28by%20ref%29))
  (CallFunction|DealDamagefromSpikes OtherActor))

(event OnComponentHit(Cone2)
  (params (HitComponent :type Primitive%20Component%20Object%20Reference) (OtherActor :type Actor%20Object%20Reference) (OtherComp :type Primitive%20Component%20Object%20Reference) (NormalImpulse :type Vector :default "0, 0, 0") (Hit :type Hit%20Result%20Structure%20%28by%20ref%29))
  (CallFunction|DealDamagefromSpikes OtherActor))

(event EventBeginPlay
  (|CallParentFunction) ; This node is disabled and will not be called.\nDrag off pins to build functionality.
)

(event Collision|EventActorBeginOverlap
  (params (OtherActor :type Actor%20Object%20Reference))
  (|CallParentFunction OtherActor) ; This node is disabled and will not be called.\nDrag off pins to build functionality.
)

(event EventTick
  (params (DeltaSeconds :type Float%20%28single-precision%29))
  (|CallParentFunction DeltaSeconds) ; This node is disabled and will not be called.\nDrag off pins to build functionality.
)

(event EventDestroyMe
  (Audio|PlaySoundatLocation "/Game/SoundFX/SpikedDevil/animals_alligator_hiss_Cue.animals_alligator_hiss_Cue" (Transformation|GetActorLocation) "0, 0, 0" 1.0 1.0 0.0 "/Game/Evgeniy/AdditionalBP/SoundAttenuation_Bullet.SoundAttenuation_Bullet" 0 0 0)
  (Variables|Default|SetSize (Transformation|GetWorldScale (Variables|Default|GetStaticMesh)))
  (bind _size (Timeline|death Play)
    (:Update
      (Transformation|SetWorldScale3D (Variables|Default|GetStaticMesh) (* _size (Variables|Default|GetSize))))
    (:Finished
      (Actor|DestroyActor))))

(fn ConstructionScript
  (|CallParentFunction))