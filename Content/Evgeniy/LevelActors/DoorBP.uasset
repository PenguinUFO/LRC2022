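; DoorBP is a level door actor that opens by hiding its mesh and disabling collision, and closes by restoring both.
; Overrides of the parent's DoIt and UndoIt call TurnIt to open or close it, and the construction script applies the Open flag.
; An older timeline-driven swing with sound remains disconnected, marked for a remake, alongside its rotation helper functions.
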(event Custom|TurnIt
  (params (Do%20we%20open%20it%20now? :type Boolean))
  (bind _staticmesh_0 (Variables|Default|GetStaticMesh_0))
  (bind _output_get (Variables|Default|SetOpen Do%20we%20open%20it%20now?))
  (Rendering|SetVisibility _staticmesh_0 (not _output_get) true)
  (if _output_get
    (Collision|SetCollisionEnabled _staticmesh_0 "NoCollision")
    (else
      (Collision|SetCollisionEnabled _staticmesh_0 "QueryAndPhysics"))))

(event EventBeginPlay
  (|CallParentFunction) ; This node is disabled and will not be called.\nDrag off pins to build functionality.
)

(event Collision|EventActorBeginOverlap
  (params (OtherActor :type Actor%20Object%20Reference))
  (|CallParentFunction OtherActor) ; This node is disabled and will not be called.\nDrag off pins to build functionality.
)

(event EventTick
  (params (DeltaSeconds :type Float%20%28single-precision%29))
  (|CallParentFunction DeltaSeconds) ; This node is disabled and will not be called.\nDrag off pins to build functionality.
)

(fn ConstructionScript
  (|CallParentFunction)
  (CallFunction|TurnIt (Variables|Default|GetOpen)))

(fn OpenorClose
  (params (FlipOrFlop :type Boolean))
  (bind _initialrotation (Variables|Default|GetInitialRotation))
  (if FlipOrFlop
    (Transformation|SetRelativeRotation (Variables|Default|GetStaticMesh_0) (Math|Rotator|MakeRotator (.roll _initialrotation) (.pitch _initialrotation) (+ (.yaw _initialrotation) (Variables|Default|GetOpenDegree))) false false)
    (else
      (Transformation|SetRelativeRotation (Variables|Default|GetStaticMesh_0) (Variables|Default|GetInitialRotation) false false))))

(fn NewDoorDegree
  (params (DeltaDegree :type Float%20%28double-precision%29))
  (bind _initialrotation (Variables|Default|GetInitialRotation))
  (if (Variables|Default|GetOpen)
    (LocalVariables|SetDelta DeltaDegree)
    (else
      (LocalVariables|SetDelta (* DeltaDegree -1.0))))
  (Transformation|SetRelativeRotation (Variables|Default|GetStaticMesh_0) (Math|Rotator|MakeRotator (.roll _initialrotation) (.pitch _initialrotation) (+ (.yaw _initialrotation) (LocalVariables|GetDelta))) false false))

(fn DoIt
  (|CallParentFunction)
  (CallFunction|TurnIt true))

(fn UndoIt
  (|CallParentFunction)
  (CallFunction|TurnIt false))