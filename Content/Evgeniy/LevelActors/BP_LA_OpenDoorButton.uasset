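; BP_LA_OpenDoorButton is a pressure button level actor that triggers linked actors when something enters its capsule collision.
; The first overlap shrinks or reshapes the button via relative scale, sets IsPressed and calls DoIt on each valid SlaveActor.
; End overlap restores the default scale and clears IsPressed once DoWeOverlapAnything returns false.
; Release does not notify the slave actors; a second DoIt loop is left unconnected.
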(event OnComponentBeginOverlap(CapsuleCollision)
  (params (OverlappedComponent :type Primitive%20Component%20Object%20Reference) (OtherActor :type Actor%20Object%20Reference) (OtherComp :type Primitive%20Component%20Object%20Reference) (OtherBodyIndex :type Integer) (bFromSweep :type Boolean) (SweepResult :type Hit%20Result%20Structure%20%28by%20ref%29))
  (if (not (Variables|Default|GetisPressed))
    (Transformation|SetRelativeScale3D (Variables|Default|GetButton) (Variables|Default|GetPressedButtonScale)) ; Сделали вид, что она нажата
    (Variables|Default|SetisPressed true) ; Записали в переменную, что она нажата
    (for _array_element (Variables|Default|GetSlaveActor)
      (Utilities|IsValid _array_element
        (:Is%20Valid
          (Default|DoIt _array_element))))))

(event OnComponentEndOverlap(CapsuleCollision)
  (params (OverlappedComponent :type Primitive%20Component%20Object%20Reference) (OtherActor :type Actor%20Object%20Reference) (OtherComp :type Primitive%20Component%20Object%20Reference) (OtherBodyIndex :type Integer))
  (if (Variables|Default|GetisPressed)
    (if (not (CallFunction|DoWeOverlapAnything?)) ; Если еще есть пересечение, значит что-то давит на нее
      (Transformation|SetRelativeScale3D (Variables|Default|GetButton) (Variables|Default|GetDefaultButtonScale)) ; Сделали вид, что она НЕ нажата
      (Variables|Default|SetisPressed false) ; Записали в переменную, что она НЕ нажата
    )))

(event EventBeginPlay
  (|CallParentFunction) ; This node is disabled and will not be called.\nDrag off pins to build functionality.
)

(event Collision|EventActorBeginOverlap
  (params (OtherActor :type Actor%20Object%20Reference))
  (|CallParentFunction OtherActor) ; This node is disabled and will not be called.\nDrag off pins to build functionality.
)

(event EventTick
  (params (DeltaSeconds :type Float%20%28single-precision%29))
  (|CallParentFunction DeltaSeconds) ; This node is disabled and will not be called.\nDrag off pins to build functionality.
)

(fn ConstructionScript
  (|CallParentFunction))