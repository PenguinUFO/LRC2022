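; A pressure button level actor that switches a linked SlaveActor on and off.
; An overlap by an actor with a valid tag shrinks or restores the button via preset scales and calls DoIt or UndoIt on the slave.
; Before releasing, a zero-length multi sphere trace on Visibility at the capsule checks that no other tagged actor still holds the button down.
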(event OnComponentBeginOverlap(CapsuleCollision)
  (params (OverlappedComponent :type Primitive%20Component%20Object%20Reference) (OtherActor :type Actor%20Object%20Reference) (OtherComp :type Primitive%20Component%20Object%20Reference) (OtherBodyIndex :type Integer) (bFromSweep :type Boolean) (SweepResult :type Hit%20Result%20Structure%20%28by%20ref%29))
  (Utilities|IsValidActor OtherActor
    (:isValid
      (if (not (Variables|GameLogic|GetisPressed))
        (Transformation|SetRelativeScale3D (Variables|Default|GetButton) (Variables|Visual|GetPressedButtonScale)) ; Сделали вид, что она нажата
        (Variables|GameLogic|SetisPressed true) ; Записали в переменную, что она нажата
        (bind _slaveactor (Variables|Default|GetSlaveActor) ; Кнопка к чему-либо подсоединена?
          (:then
            (Default|DoIt _slaveactor) ; Запускай шарманку - что там должно делать устройство, к которому кнопка подключена
          )
          (:else))))))

(event OnComponentEndOverlap(CapsuleCollision)
  (params (OverlappedComponent :type Primitive%20Component%20Object%20Reference) (OtherActor :type Actor%20Object%20Reference) (OtherComp :type Primitive%20Component%20Object%20Reference) (OtherBodyIndex :type Integer))
  (Utilities|IsValidActor OtherActor
    (:isValid
      (if (Variables|GameLogic|GetisPressed)
        (if (not (CallFunction|DoWeOverlapAnything?)) ; Если еще есть пересечение, значит что-то давит на нее
          (Transformation|SetRelativeScale3D (Variables|Default|GetButton) (Variables|Visual|GetDefaultButtonScale)) ; Сделали вид, что она НЕ нажата
          (Variables|GameLogic|SetisPressed false) ; Записали в переменную, что она НЕ нажата
          (bind _slaveactor (Variables|Default|GetSlaveActor) ; Кнопка к чему-либо подсоединена?
            (:then
              (Default|UndoIt _slaveactor) ; Выключай шарманку.
            )
            (:else)))))))

(event EventBeginPlay
  (|CallParentFunction))

(event Collision|EventActorBeginOverlap
  (params (OtherActor :type Actor%20Object%20Reference))
  (|CallParentFunction OtherActor) ; This node is disabled and will not be called.\nDrag off pins to build functionality.
)

(event EventTick
  (params (DeltaSeconds :type Float%20%28single-precision%29))
  (|CallParentFunction DeltaSeconds) ; This node is disabled and will not be called.\nDrag off pins to build functionality.
)

(fn ConstructionScript
  (|CallParentFunction))

(fn DoWeOverlapAnything?
  (bind _capsulecollision (Variables|Default|GetCapsuleCollision))
  (bind _returnvalue (Transformation|GetWorldLocation _capsulecollision))
  (bind _outhits (Collision|MultiSphereTraceByChannel _returnvalue _returnvalue 3e+01 "TraceTypeQuery1" false 0 "None"))
  (for _array_element _outhits
    (Utilities|IsValidActor (.HitActor (Collision|BreakHitResult _array_element))
      (:isValid
        (return true))))
  (return false))