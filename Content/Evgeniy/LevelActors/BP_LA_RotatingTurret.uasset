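; BP_LA_RotatingTurret is a level actor turret that fires missiles and switches between two fixed facings.
; A looping timer started at BeginPlay calls Shoot while IsOn is true, spawning a half-scale missile at SpawnPoint along the mesh's rotation with the configured speed.
; DoIt and UndoIt overrides snap the mesh to TriggerAngle or back to InitialAngle, redirecting later shots.
; DestroyMe runs the parent Destroy logic, then removes the actor.
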(event Custom|ShootingOnTime
  (if (Variables|Default|GetIsOn)
    (CallFunction|Shoot)))

(event EventBeginPlay
  (|CallParentFunction)
  (Utilities|Time|SetTimerbyEvent (delegate Custom|ShootingOnTime) (Variables|Default|GetDelayBetweenShoots) true))

(event Collision|EventActorBeginOverlap
  (params (OtherActor :type Actor%20Object%20Reference))
  (|CallParentFunction OtherActor) ; This node is disabled and will not be called.\nDrag off pins to build functionality.
)

(event EventTick
  (params (DeltaSeconds :type Float%20%28single-precision%29))
  (|CallParentFunction DeltaSeconds) ; This node is disabled and will not be called.\nDrag off pins to build functionality.
)

(event EventDestroyMe
  (CallFunction|Destroy))

(fn ConstructionScript
  (|CallParentFunction))

(fn Shoot
  (Game|SpawnActorfromClass (Variables|Default|GetMissle) (Math|Transform|MakeTransform (+ (Transformation|GetWorldLocation (Variables|Default|GetSpawnPoint)) "") (Transformation|GetWorldRotation (Variables|Default|GetStaticMesh)) "0.500000,0.500000,0.500000") "Undefined" self (Variables|Default|GetMissleSpeed) 0))

(fn DoIt
  (|CallParentFunction)
  (Transformation|SetWorldRotation (Variables|Default|GetStaticMesh) (Variables|Default|GetTriggerAngle) false false))

(fn UndoIt
  (|CallParentFunction)
  (Transformation|SetWorldRotation (Variables|Default|GetStaticMesh) (Variables|Default|GetInitialAngle) false false))

(fn Destroy
  (|CallParentFunction)
  (Actor|DestroyActor))