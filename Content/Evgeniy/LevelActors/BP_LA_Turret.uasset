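; BP_LA_Turret is a level actor turret that fires missiles at a fixed interval while switched on.
; A looping timer started on BeginPlay calls Shoot whenever IsOn is set, spawning a half-scale Missle just below the static mesh, with its rotation and the configured speed.
; Overrides of the parent's DoIt and UndoIt toggle firing, and Destroy removes the actor.
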(event Custom|ShootingOnTime
  (if (Variables|Default|GetIsOn)
    (CallFunction|Shoot)))

(event EventBeginPlay
  (|CallParentFunction)
  (Utilities|Time|SetTimerbyEvent (delegate Custom|ShootingOnTime) (Variables|Default|GetDelayBetweenShoots) true))

(event Collision|EventActorBeginOverlap
  (params (OtherActor :type Actor%20Object%20Reference))
  (|CallParentFunction OtherActor) ; This node is disabled and will not be called.\nDrag off pins to build functionality.
)

(event EventTick
  (params (DeltaSeconds :type Float%20%28single-precision%29))
  (|CallParentFunction DeltaSeconds) ; This node is disabled and will not be called.\nDrag off pins to build functionality.
)

(event EventDestroyMe
  (CallFunction|Destroy))

(fn ConstructionScript
  (|CallParentFunction))

(fn Shoot
  (bind _staticmesh (Variables|Default|GetStaticMesh))
  (Game|SpawnActorfromClass (Variables|Default|GetMissle) (Math|Transform|MakeTransform (+ (Transformation|GetWorldLocation _staticmesh) "0.000000,0,-80.000000") (Transformation|GetWorldRotation _staticmesh) "0.500000,0.500000,0.500000") "Undefined" self (Variables|Default|GetMissleSpeed) 0))

(fn DoIt
  (|CallParentFunction)
  (Variables|Default|SetIsOn true))

(fn UndoIt
  (|CallParentFunction)
  (Variables|Default|SetIsOn false))

(fn Destroy
  (|CallParentFunction)
  (Actor|DestroyActor))