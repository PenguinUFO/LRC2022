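; BP_LA_Camera is a security camera level actor that closes a linked door while it spots intruders.
; ConeOfSight overlap events keep a duplicate-free ActorsInSight list, with no filter on actor type.
; Each list change re-evaluates the door, calling DoIt on SlaveActor to close it, or UndoIt to reopen it once the list is empty.
; Tick prints a debug message for every spotted actor.
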(event OnComponentBeginOverlap(ConeOfSight)
  (params (OverlappedComponent :type Primitive%20Component%20Object%20Reference) (OtherActor :type Actor%20Object%20Reference) (OtherComp :type Primitive%20Component%20Object%20Reference) (OtherBodyIndex :type Integer) (bFromSweep :type Boolean) (SweepResult :type Hit%20Result%20Structure%20%28by%20ref%29))
  (Utilities|FlowControl|Sequence
    (:then_0
      (CallFunction|AddIntrudertoActorsinSightList OtherActor))
    (:then_1
      (CallFunction|UpdateDoorState))))

(event OnComponentEndOverlap(ConeOfSight)
  (params (OverlappedComponent :type Primitive%20Component%20Object%20Reference) (OtherActor :type Actor%20Object%20Reference) (OtherComp :type Primitive%20Component%20Object%20Reference) (OtherBodyIndex :type Integer))
  (Utilities|FlowControl|Sequence
    (:then_0
      (CallFunction|RemoveIntruderfromActorsinSightList OtherActor))
    (:then_1
      (CallFunction|UpdateDoorState))))

(event EventBeginPlay
  (|CallParentFunction) ; This node is disabled and will not be called.\nDrag off pins to build functionality.
)

(event Collision|EventActorBeginOverlap
  (params (OtherActor :type Actor%20Object%20Reference))
  (|CallParentFunction OtherActor) ; This node is disabled and will not be called.\nDrag off pins to build functionality.
)

(event EventTick
  (params (DeltaSeconds :type Float%20%28single-precision%29))
  (|CallParentFunction DeltaSeconds)
  (for _array_element (Variables|Default|GetActorsInSight)
    (Development|PrintString (Utilities|String|ToString(Text) (Utilities|Text|FormatText "I Spotted the {intruder}" _array_element)) true true "(R=0.054941,G=0.000000,B=0.708333,A=1.000000)" 0.0)))

(fn ConstructionScript
  (|CallParentFunction))

(fn DoWeSpotSomeone?
  (if (== (Utilities|Array|Length (Variables|Default|GetActorsInSight)) 0)
    (return false)
    (else
      (return true))))

(fn AddIntrudertoActorsinSightList
  (params (Intruder :type Actor%20Object%20Reference%20%28by%20ref%29))
  (if (not (Utilities|Array|ContainsItem (Variables|Default|GetActorsInSight) Intruder))
    (Utilities|Array|Add (Variables|Default|GetActorsInSight) Intruder)))

(fn RemoveIntruderfromActorsinSightList
  (params (Intruder :type Actor%20Object%20Reference%20%28by%20ref%29))
  (if (Utilities|Array|ContainsItem (Variables|Default|GetActorsInSight) Intruder)
    (Utilities|Array|RemoveItem (Variables|Default|GetActorsInSight) Intruder)))

(fn UpdateDoorState
  (bind _slaveactor (Variables|Default|GetSlaveActor))
  (if (CallFunction|DoWeSpotSomeone?)
    (Default|DoIt _slaveactor) ; Закрыть дверь!
    (else
      (Default|UndoIt _slaveactor) ; Открыть дверь
    )))