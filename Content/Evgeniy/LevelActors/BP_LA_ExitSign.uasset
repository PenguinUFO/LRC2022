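; Exit sign level actor that signals with a bell sound and a blinking green light when its DoIt function is triggered.
; DoIt extends the parent's implementation by playing an elevator bell at the actor's location, turning the point light green and calling the blink event.
; A timeline drives the blink, scaling its intensity curve by a maximum intensity variable on each update.
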(event Custom|BlincWithLight
  (bind _lightintencity (Timeline|greenLightBlinking Play)
    (:Update
      (Rendering|Components|Light|SetIntensity (Variables|Default|GetPointLight) (* _lightintencity (Variables|Default|GetLightMaxIntensity))))))

(event EventBeginPlay
  (|CallParentFunction) ; This node is disabled and will not be called.\nDrag off pins to build functionality.
)

(event Collision|EventActorBeginOverlap
  (params (OtherActor :type Actor%20Object%20Reference))
  (|CallParentFunction OtherActor) ; This node is disabled and will not be called.\nDrag off pins to build functionality.
)

(event EventTick
  (params (DeltaSeconds :type Float%20%28single-precision%29))
  (|CallParentFunction DeltaSeconds) ; This node is disabled and will not be called.\nDrag off pins to build functionality.
)

(fn ConstructionScript
  (|CallParentFunction))

(fn DoIt
  (|CallParentFunction)
  (Audio|PlaySoundatLocation "/Game/SoundFX/Teleport/Elevator_bell_small_001.Elevator_bell_small_001" (Transformation|GetActorLocation) "0, 0, 0" 1.0 1.0 0.0 "/Game/Evgeniy/AdditionalBP/SoundAttenuation_Bullet.SoundAttenuation_Bullet" 0 0 0)
  (Rendering|Components|Light|SetLightColor (Variables|Default|GetPointLight) "(R=0.000000,G=0.385417,B=0.065387,A=1.000000)" true)
  (CallFunction|BlincwithLight))