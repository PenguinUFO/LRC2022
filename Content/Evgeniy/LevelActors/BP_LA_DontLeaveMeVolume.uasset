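; BP_LA_DontLeaveMeVolume is a level trigger that retrieves a companion the player left behind.
; When the player enters its box, it waits, then queries the listed seeker zones for the specified left-behind actor.
; A found companion teleports to a preset location and speaks a plea, then the volume destroys itself, optionally removing all seekers.
; The construction script sizes the box from exposed Y and Z values.
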(event OnComponentBeginOverlap(Box)
  (params (OverlappedComponent :type Primitive%20Component%20Object%20Reference) (OtherActor :type Actor%20Object%20Reference) (OtherComp :type Primitive%20Component%20Object%20Reference) (OtherBodyIndex :type Integer) (bFromSweep :type Boolean) (SweepResult :type Hit%20Result%20Structure%20%28by%20ref%29))
  (if (== OtherActor (Game|GetPlayerCharacter 0))
    (Utilities|FlowControl|Delay (Variables|Default|GetHow%20Long%20to%20Wait%20Before%20search))
    ;[1 1 1] ищем шарик в указанных зонах
    (bind _array_element (Utilities|Array|ForEachLoopwithBreak (Variables|Default|Getwhere%20could%20we%20leave%20it) :!label _label)
      (:LoopBody
        (Utilities|IsValid _array_element
          (:Is%20Valid
            (bind (_actors _someonehere) (Default|CheckforPresensOf _array_element (Variables|Default|GetWho%20is%20leaved)))
            (bind _output_get (Variables|Default|SetDo%20we%20finde%20it? _someonehere))
            (if _output_get
              (bind _asbp_companion (Utilities|Casting|CastToBP_Companion (Utilities|Array|Get(acopy) _actors)))
              (Variables|Default|SetLostedActor _asbp_companion)
              (goto _label Break)))))
      (:Completed
        ;[1 1 1] Нашли шарик - тяни его к игроку!
        (if (Variables|Default|GetDo%20we%20finde%20it?)
          (Transformation|SetActorLocation (Variables|Default|GetLostedActor) (Variables|Default|GetWhere%20we%20should%20place%20him?) false false)
          (Default|Speak (Variables|Default|GetLostedActor) "Please, don't leave me here! Take me with you!" "/Game/SoundFX/Companion/CompanionVoice/CompanionVoice_Cue.CompanionVoice_Cue")
          ;[1 1 1] убираем все лишнее с карты
          (if (Variables|Default|GetDestroyAllSeekers?)
            (for _array_element_2 (Variables|Default|Getwhere%20could%20we%20leave%20it)
              (Actor|DestroyActor _array_element_2)))
          (Actor|DestroyActor))))))

(event EventBeginPlay
  (|CallParentFunction) ; This node is disabled and will not be called.\nDrag off pins to build functionality.
)

(event Collision|EventActorBeginOverlap
  (params (OtherActor :type Actor%20Object%20Reference))
  (|CallParentFunction OtherActor) ; This node is disabled and will not be called.\nDrag off pins to build functionality.
)

(event EventTick
  (params (DeltaSeconds :type Float%20%28single-precision%29))
  (|CallParentFunction DeltaSeconds) ; This node is disabled and will not be called.\nDrag off pins to build functionality.
)

(fn ConstructionScript
  (|CallParentFunction)
  (Transformation|SetWorldScale3D (Variables|Default|GetBox) (Math|Vector|MakeVector 3.0 (Variables|World|GetBoxY) (Variables|World|GetBoxZ))))

(fn ReleaseAllFinders)