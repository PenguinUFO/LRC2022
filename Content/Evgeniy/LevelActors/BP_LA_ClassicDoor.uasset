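; BP_LA_ClassicDoor is a swinging door level actor that opens when the player character overlaps its Box trigger.
; The overlap calls the inherited DoIt, which runs the parent logic, then OpenTheDoor sets IsOpen and plays DoorTimeline to add yaw scaled by OpenDegree.
; The construction script applies the configurable mesh and caches its world rotation as the closed pose.
; The graph has no closing logic.
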(event OnComponentBeginOverlap(Box)
  (params (OverlappedComponent :type Primitive%20Component%20Object%20Reference) (OtherActor :type Actor%20Object%20Reference) (OtherComp :type Primitive%20Component%20Object%20Reference) (OtherBodyIndex :type Integer) (bFromSweep :type Boolean) (SweepResult :type Hit%20Result%20Structure%20%28by%20ref%29))
  (if (and (== OtherActor (Game|GetPlayerCharacter 0)) (not (Variables|Default|GetisOpen)))
    (CallFunction|DoIt)))

(event Custom|OpenTheDoor
  (bind _initialrotation (Variables|Default|GetInitialRotation))
  (Variables|Default|SetisOpen true)
  (bind _newtrack_0 (Timeline|DoorTimeline Play)
    (:Update
      (Transformation|SetWorldRotation (Variables|Default|GetStaticMesh) (Math|Rotator|MakeRotator (.roll _initialrotation) (.pitch _initialrotation) (+ (* _newtrack_0 (Variables|Default|GetOpenDegree)) (.yaw _initialrotation))) false false))))

(event EventBeginPlay
  (|CallParentFunction) ; This node is disabled and will not be called.\nDrag off pins to build functionality.
)

(event Collision|EventActorBeginOverlap
  (params (OtherActor :type Actor%20Object%20Reference))
  (|CallParentFunction OtherActor) ; This node is disabled and will not be called.\nDrag off pins to build functionality.
)

(event EventTick
  (params (DeltaSeconds :type Float%20%28single-precision%29))
  (|CallParentFunction DeltaSeconds) ; This node is disabled and will not be called.\nDrag off pins to build functionality.
)

(fn ConstructionScript
  (|CallParentFunction)
  (Components|StaticMesh|SetStaticMesh (Variables|Default|GetStaticMesh) (Variables|Default|GetMesh))
  (Variables|Default|SetInitialRotation (Transformation|GetWorldRotation (Variables|Default|GetStaticMesh))))

(fn DoIt
  (|CallParentFunction)
  (CallFunction|OpentheDoor))